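; Tank variant of the flying enemy that can carry a turret, built on a parent Blueprint that it tunes with a collision radius for obstacle avoidance and its own death delay.
; On BeginPlay it optionally spawns a BP_BasicTurret at the ship's TurretSocket, attaches it and copies in tags plus weapon, projectile, damage and fire-rate settings.
; The destroyed event flags the tank and removes the turret if it is still alive.
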(event EventBeginPlay
  (|CallParentFunction)
  ;[1 1 1] Collision radius used for obstacle avoidance
  (Variables|Default|SetCollisionSphereRadius 3e+03)
  ;[1 1 1] Spawn turret?
  (if (Variables|Setup-Turret|GetSpawnTurret?)
    ;[1 1 1] Spawn the turret
    (CallFunction|EventSpawnTurrets)))

(fn ConstructionScript
  (|CallParentFunction)
  ;[1 1 1] Set DM_DeathDelay to 10 - default in parentBP class
  (Variables|Default|SetDM_DeathDelay 1e+01))

(event Custom|EventSpawnTurrets
  (bind _ship (Variables|Default|GetShip))
  ;[1 1 1] Spawn turret and attach to socket
  (bind _returnvalue (Game|SpawnActorfromClass "/Game/ASST/Blueprints/Characters/Enemies/GroundEnemies/BP_BasicTurret.BP_BasicTurret_C" (Math|Transform|MakeTransform (Transformation|GetSocketLocation _ship "TurretSocket") (Transformation|GetWorldRotation _ship)) "Undefined" "OverrideRootScale" 0 0))
  (bind _output_get (Variables|Setup-Turret|SetTurretRef _returnvalue))
  (Transformation|AttachActorToActor _output_get self "TurretSocket" "KeepWorld" "KeepWorld" "KeepWorld" true)
  ;[1 1 1] Set 'Spawned' tag to turret
  (Variables|/Script/Engine.Actor|SetTags (Variables|Setup-Turret|GetTurretRef) (Variables|Setup-Turret|GetTurretTags))
  ;[1 1 1] Setup Turret Preferences
  (Variables|/Game/ASST/Blueprints/Characters/Enemies/GroundEnemies/BP_BasicTurret.BP_BasicTurret_C|SetWeaponType (Variables|Setup-Turret|GetTurretRef) (Variables|Setup-Turret|GetTurretWeaponType))
  (Variables|/Game/ASST/Blueprints/Characters/Enemies/GroundEnemies/BP_BasicTurret.BP_BasicTurret_C|SetProjectileType (Variables|Setup-Turret|GetTurretRef) (Variables|Setup-Turret|GetTurretProjectileType))
  (Variables|/Game/ASST/Blueprints/Characters/Enemies/GroundEnemies/BP_BasicTurret.BP_BasicTurret_C|SetDamageType (Variables|Setup-Turret|GetTurretRef) (Variables|Setup-Turret|GetTurretDamageType))
  (Variables|/Game/ASST/Blueprints/Characters/Enemies/GroundEnemies/BP_BasicTurret.BP_BasicTurret_C|SetFireRate (Variables|Setup-Turret|GetTurretRef) (Variables|Setup-Turret|GetTurretFireRate)))

(event EventEventDestroyed
  (Variables|Default|SetDestroyed true)
  ;[1 1 1] Check if turret is valid (still alive)
  (if (Utilities|IsValid (Variables|Setup-Turret|GetTurretRef))
    ;[1 1 1] Destroy turret
    (Actor|DestroyActor (Variables|Setup-Turret|GetTurretRef))))