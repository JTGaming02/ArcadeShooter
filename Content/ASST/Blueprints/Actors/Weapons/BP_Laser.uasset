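; BP_Laser is a laser projectile that damages non-player actors it hits and expires after a set lifetime.
; Its construction script sets the projectile movement velocity and actor tags, and BeginPlay makes the mesh ignore the player pawn when moving.
; A mesh hit on an actor without the Player tag applies point damage, spawns explosion particles and sound, then destroys the laser after a brief delay.
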(event OnComponentHit(LaserMesh)
  (params (HitComponent :type Primitive%20Component%20Object%20Reference) (OtherActor :type Actor%20Object%20Reference) (OtherComp :type Primitive%20Component%20Object%20Reference) (NormalImpulse :type Vector :default "0, 0, 0") (Hit :type Hit%20Result%20Structure%20%28by%20ref%29))
  (Variables|Default|SetHitComponent HitComponent)
  (bind _output_get (Variables|Default|SetOtherActor OtherActor))
  (Utilities|IsValid _output_get
    (:Is%20Valid
      ;[1 1 1] Do not hit the Player
      (if (not (Actor|ActorHasTag (Variables|Default|GetOtherActor) "Player"))
        ;[1 1 1] Apply point damage
        (Game|Damage|ApplyPointDamage (Variables|Default|GetOtherActor) (Variables|Setup|GetBaseDamage) (* (.ImpactNormal (Collision|BreakHitResult Hit)) -1.0) Hit 0 self)
        ;[1 1 1] Spawn emitter at hit location
        (Effects|SpawnEmitteratLocation (Variables|Setup|GetExplosionParticles) (Transformation|GetWorldLocation (Variables|Default|GetHitComponent)))
        ;[1 1 1] Play explosion sound
        (Audio|PlaySoundatLocation (Variables|Setup|GetExplosionSound) (Transformation|GetWorldLocation (Variables|Default|GetHitComponent)) "0, 0, 0" 1.0 1.0 0.0 0 0 0 0)
        ;[1 1 1] Wait for 0.2secs and destroy the actor
        (Utilities|FlowControl|Delay 0.1)
        (Actor|DestroyActor)))))

(event EventBeginPlay
  ;[1 1 1] Set Laser lifespan
  (Actor|SetLifeSpan (Variables|Default|GetTimeToLive))
  ;[1 1 1] Ignore player pawn
  (Collision|IgnoreActorwhenMoving (Variables|Default|GetLaserMesh) (Game|Player|GetPlayerPawn 0) true))

(fn ConstructionScript
  ;[1 1 1] Set velocity
  (Variables|/Script/Engine.MovementComponent|SetVelocity (Variables|Default|GetProjectileMovement) (Variables|Setup|GetProjectileVelocity))
  ;[1 1 1] Set actor tags
  (Variables|Default|SetTags (Variables|Default|GetActorTags)))