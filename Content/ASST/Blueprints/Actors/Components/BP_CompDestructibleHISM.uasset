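; Actor component that makes each instance of its owner's Hierarchical Instanced Static Mesh destructible when the owner is hit.
; BeginPlay fills a per-instance health map; each hit takes one point, after a short delay, from the first instance found near the impact.
; At zero health, it swaps the instance for a Geometry Collection actor, fractures it with a spawned master field, plays a sound and optionally removes debris later.
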(event Custom|EventHit
  (params (SelfActor :type Actor%20Object%20Reference) (OtherActor :type Actor%20Object%20Reference) (NormalImpulse :type Vector) (Hit :type Hit%20Result%20Structure%20%28by%20ref%29))
  (bind (_bblockinghit _binitialoverlap _time _distance _location _impactpoint _normal _impactnormal) (Collision|BreakHitResult Hit))
  ;[1 1 1] Bind OnActorHit event
  ;[1 1 1] Save the hit location and normal
  (Variables|Default|SetHitLocation _impactpoint)
  (Variables|Default|SetImpactNormal _impactnormal)
  ;[1 1 1] Get Instance Hit
  (if (Utilities|Array|IsNotEmpty (Class|InstancedStaticMeshComponent|GetInstancesOverlappingSphere (Actor|GetComponentbyClass (Components|GetOwner) "/Script/Engine.HierarchicalInstancedStaticMeshComponent") (Variables|Default|GetHitLocation) 1e+03 true))
    (Variables|Default|SetInstanceHit (Utilities|Array|Get(acopy) (Class|InstancedStaticMeshComponent|GetInstancesOverlappingSphere (Actor|GetComponentbyClass (Components|GetOwner) "/Script/Engine.HierarchicalInstancedStaticMeshComponent") (Variables|Default|GetHitLocation) 1e+03 true)))
    ;[1 1 1] Apply damage to the instance
    (CallFunction|EventApplyDamage)))

(event EventBeginPlay
  ;[1 1 1] Populate health map
  (CallFunction|EventPopulateHealthMap)
  ;[1 1 1] Bind OnActorHit event
  (Collision|BindEventtoOnActorHit (Components|GetOwner) (delegate Custom|EventHit)))

(event Custom|EventApplyDamage
  (bind _destructiondelay (Variables|Setup|GetDestructionDelay))
  (Utilities|FlowControl|Delay 0.2)
  ;[1 1 1] Reduce Health of instance by 1 hit
  (Utilities|Map|Add (Variables|Default|GetInstanceHealthMap) (Variables|Default|GetInstanceHit) (- (.Value (Utilities|Map|Find (Variables|Default|GetInstanceHealthMap) (Variables|Default|GetInstanceHit))) 1))
  ;[1 1 1] Check if the instance's health reached 0
  (if (<= (.Value (Utilities|Map|Find (Variables|Default|GetInstanceHealthMap) (Variables|Default|GetInstanceHit))) 0)
    ;[1 1 1] Save instance transform before removing it
    (Variables|Default|SetNewDMTransform (.OutInstanceTransform (Components|InstancedStaticMesh|GetInstanceTransform (Actor|GetComponentbyClass (Components|GetOwner) "/Script/Engine.HierarchicalInstancedStaticMeshComponent") (Variables|Default|GetInstanceHit) true)))
    ;[1 1 1] Spawn the GC Building class
    (Utilities|FlowControl|Delay 0.1)
    (bind _returnvalue (Game|SpawnActorfromClass (Variables|Setup|GetBuildingGC_Class) (Variables|Default|GetNewDMTransform) "AlwaysSpawn" 0 0))
    (Variables|Default|SetBuildingGC _returnvalue)
    ;[1 1 1] Remove instance
    (Class|InstancedStaticMeshComponent|RemoveInstance (Actor|GetComponentbyClass (Components|GetOwner) "/Script/Engine.HierarchicalInstancedStaticMeshComponent") (Variables|Default|GetInstanceHit))
    ;[1 1 1] Remove map element
    (Utilities|Map|Remove (Variables|Default|GetInstanceHealthMap) (Variables|Default|GetInstanceHit))
    ;[1 1 1] Spawn a Master Field to apply strain to the GC
    (bind _returnvalue_2 (Game|SpawnActorfromClass "/Engine/EditorResources/FieldNodes/FS_MasterField.FS_MasterField_C" (Math|Transform|MakeTransform (Variables|Default|GetHitLocation) "0, 0, 0" "5.000000,5.000000,5.000000") "Undefined" 0 0))
    (Variables|Default|SetSpawnedField _returnvalue_2)
    (Variables|/Engine/EditorResources/FieldNodes/FS_MasterField.FS_MasterField_C|SetActivationType (Variables|Default|GetSpawnedField) "NewEnumerator4")
    ;[1 1 1] Set the Radial and Directional Magnitude
    (Variables|/Engine/EditorResources/FieldNodes/FS_MasterField.FS_MasterField_C|SetRadial%20Magnitude (Variables|Default|GetSpawnedField) (Variables|Setup|GetRadial%20Magnitude))
    (Variables|/Engine/EditorResources/FieldNodes/FS_MasterField.FS_MasterField_C|SetDirectionalMagnitude (Variables|Default|GetSpawnedField) (Variables|Setup|GetDirectional%20Magnitude))
    ;[1 1 1] Trigger the Field
    (Default|CETrigger (Variables|Default|GetSpawnedField))
    ;[1 1 1] Play destruction sound
    (Audio|PlaySoundatLocation (Variables|Setup|GetDestructionSound) (Variables|Default|GetHitLocation) "0, 0, 0" 1.0 1.0 0.0 0 0 0 0)
    ;[1 1 1] Destroy Component, if appropriate
    (if (Variables|Setup|GetDestroyDebris?)
      (if (Utilities|IsValid (Actor|GetComponentbyClass (Variables|Default|GetBuildingGC) "/Game/ASST/Blueprints/Actors/Components/BP_CompDelayedDeath.BP_CompDelayedDeath_C"))
        (Default|EventDelayDeath (Actor|GetComponentbyClass (Variables|Default|GetBuildingGC) "/Game/ASST/Blueprints/Actors/Components/BP_CompDelayedDeath.BP_CompDelayedDeath_C") _destructiondelay)
        (else
          (Utilities|FlowControl|Delay _destructiondelay)
          (Actor|DestroyActor (Variables|Default|GetBuildingGC)))))))

(event Custom|EventPopulateHealthMap
  ;[1 1 1] Go through all instances on the HISM component
  (for _index (range 0 (- (Components|InstancedStaticMesh|GetInstanceCount (Actor|GetComponentbyClass (Components|GetOwner) "/Script/Engine.HierarchicalInstancedStaticMeshComponent")) 1))
    ;[1 1 1] Create a new map entry for each instance and save the InstanceHealth
    (Utilities|Map|Add (Variables|Default|GetInstanceHealthMap) _index (Variables|Setup|GetInstanceHealth))))