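; BP_DifficultyManager is an actor that applies a Difficulty setting to enemies in the level.
; On BeginPlay, if Active, it waits briefly so enemies can spawn, then fires EventSetDifficulty.
; That event finds turrets, flying enemies and two bosses by class, each behind an include flag, and passes Difficulty to their own EventSetDifficulty.
; Every turret and flying enemy receives it, but only the first instance of each boss class does.
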(event EventBeginPlay
  ;[1 1 1] If the blueprint is active, call EventSetDifficulty after a brief delay (delay is used to give time to enemies to spawn in the level)
  (if (Variables|Setup|GetActive)
    (Utilities|FlowControl|Delay 0.5)
    (CallFunction|EventSetDifficulty)))

(fn ConstructionScript)

(event Custom|EventSetDifficulty
  (Utilities|FlowControl|Sequence
    (:then_0
      ;[1 1 1] Set Turret difficulty
      (if (Variables|Setup|GetIncludeTurrets?)
        (bind _outactors (Actor|GetAllActorsOfClass "/Game/ASST/Blueprints/Characters/Enemies/GroundEnemies/BP_BasicTurret.BP_BasicTurret_C"))
        (for _array_element _outactors
          (Default|EventSetDifficulty _array_element (Variables|Setup|GetDifficulty)))))
    (:then_1
      ;[1 1 1] Set Flying Enemies difficulty
      (if (Variables|Setup|GetIncludeFlyingEnemies?)
        (bind _outactors_2 (Actor|GetAllActorsOfClass "/Game/ASST/Blueprints/Characters/Enemies/FlyingEnemies/BP_FlyingEnemyBase.BP_FlyingEnemyBase_C"))
        (for _array_element_2 _outactors_2
          (Default|EventSetDifficulty _array_element_2 (Variables|Setup|GetDifficulty)))))
    (:then_2
      ;[1 1 1] Set Boss1 difficulty
      (if (Variables|Setup|GetIncludeBoss1?)
        (bind _outactors_3 (Actor|GetAllActorsOfClass "/Game/ASST/Blueprints/Characters/Enemies/Bosses/Boss1/BP_Boss1.BP_Boss1_C"))
        (if (Utilities|Array|IsValidIndex _outactors_3)
          (Default|EventSetDifficulty (Utilities|Array|Get(acopy) _outactors_3) (Variables|Setup|GetDifficulty)))))
    (:then_3
      ;[1 1 1] Set Boss 2 difficulty
      (if (Variables|Setup|GetIncludeBoss2?)
        (bind _outactors_4 (Actor|GetAllActorsOfClass "/Game/ASST/Blueprints/Characters/Enemies/Bosses/Boss2/BP_Boss2.BP_Boss2_C"))
        (if (Utilities|Array|IsValidIndex _outactors_4)
          (Default|EventSetDifficulty (Utilities|Array|Get(acopy) _outactors_4) (Variables|Setup|GetDifficulty)))))))